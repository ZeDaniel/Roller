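; BP_BaseLevel is the player-controlled level of a roller game, turning input into rotation of the level's Sphere component.
; On BeginPlay it registers an Enhanced Input mapping context with its player controller.
; Three input actions apply negated, delta-time-scaled world pitch, yaw and roll to the Sphere using RotateRate.
; Restart calls the roller game instance, while pause input toggles pause through the game mode.
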(event `self.ReceiveBeginPlay`
  ;[1 1 1] Set player controller mapping context
  (bind _asplayer_controller (cast `PlayerController` (`self.GetController`)))
  (`EnhancedInputSubsystemInterface.AddMappingContext` (pcsubsystem `EnhancedInputLocalPlayerSubsystem` _asplayer_controller) "/Game/Input/MapController.MapController" 0 (struct)))

(event `self.ReceiveTick`
  (params (DeltaSeconds :type "Float (single-precision)")))

(event `EnhancedInput|/Game/Input/RotateForward`
  (params (ActionValue :type "Float (double-precision)") (ElapsedSeconds :type "Float (double-precision)") (TriggeredSeconds :type "Float (double-precision)") (InputAction :type "InputAction Object Reference" :default "/Game/Input/RotateForward.RotateForward"))
  ;[1 1 1] Rotate world pitch
  (:`Triggered`
    (`SceneComponent.K2_AddWorldRotation` (`self.Sphere`) (`KismetMathLibrary.MakeRotator` 0.0 (* (* (* ActionValue (`self.RotateRate`)) (`GameplayStatics.GetWorldDeltaSeconds`)) -1.0)) false false)))

(event `EnhancedInput|/Game/Input/RotateLeft`
  (params (ActionValue :type "Float (double-precision)") (ElapsedSeconds :type "Float (double-precision)") (TriggeredSeconds :type "Float (double-precision)") (InputAction :type "InputAction Object Reference" :default "/Game/Input/RotateLeft.RotateLeft"))
  ;[1 1 1] Rotate world yaw
  (:`Triggered`
    (`SceneComponent.K2_AddWorldRotation` (`self.Sphere`) (`KismetMathLibrary.MakeRotator` 0.0 0.0 (* (* (* ActionValue (`self.RotateRate`)) (`GameplayStatics.GetWorldDeltaSeconds`)) -1.0)) false false)))

(event `EnhancedInput|/Game/Input/RollLeft`
  (params (ActionValue :type "Float (double-precision)") (ElapsedSeconds :type "Float (double-precision)") (TriggeredSeconds :type "Float (double-precision)") (InputAction :type "InputAction Object Reference" :default "/Game/Input/RollLeft.RollLeft"))
  ;[1 1 1] Rotate world roll
  (:`Triggered`
    (`SceneComponent.K2_AddWorldRotation` (`self.Sphere`) (`KismetMathLibrary.MakeRotator` (* (* (* ActionValue (`self.RotateRate`)) (`GameplayStatics.GetWorldDeltaSeconds`)) -1.0)) false false)))

(event `EnhancedInput|/Game/Input/Restart`
  (params (ActionValue :type Boolean) (ElapsedSeconds :type "Float (double-precision)") (TriggeredSeconds :type "Float (double-precision)") (InputAction :type "InputAction Object Reference" :default "/Game/Input/Restart.Restart"))
  (:`Triggered`
    (bind _asbp_roller_game_instance (cast `/Game/Blueprints/BP_RollerGameInstance` (`GameplayStatics.GetGameInstance`)))
    (`/Game/Blueprints/BP_RollerGameInstance.RestartGame` _asbp_roller_game_instance)))

(event `EnhancedInput|/Game/Input/IA_Pause`
  (params (ActionValue :type Boolean) (ElapsedSeconds :type "Float (double-precision)") (TriggeredSeconds :type "Float (double-precision)") (InputAction :type "InputAction Object Reference" :default "/Game/Input/IA_Pause.IA_Pause"))
  (:`Triggered`
    (bind _asbp_roller_game_mode (cast `/Game/Blueprints/BP_RollerGameMode` (`GameplayStatics.GetGameMode`)))
    (if (`/Game/Blueprints/BP_RollerGameMode.GamePaused` _asbp_roller_game_mode)
      (`/Game/Blueprints/BP_RollerGameMode.UnPauseGame` _asbp_roller_game_mode)
      (else
        (`/Game/Blueprints/BP_RollerGameMode.PauseGame` _asbp_roller_game_mode)))))

(fn `UserConstructionScript`)