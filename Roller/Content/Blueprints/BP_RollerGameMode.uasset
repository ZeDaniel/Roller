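; Game mode for a roller game that handles level startup and the win screen.
; On begin play it shows controls and level widgets, locks pawn input during a short delay, then blends view to the player camera.
; It snaps the level root onto the BaseLevel pawn, restores input and sets the game instance's target score from the count of targets.
; EndGame adds the win widget to the viewport.
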(event `self.ReceiveBeginPlay`
  (bind _returnvalue (`|CreateWidget` "/Game/Blueprints/BP_ControlsWidget.BP_ControlsWidget_C"))
  ;[1 1 1] Handle level startup
  (`UserWidget.AddToViewport` _returnvalue 0)
  (bind _asbp_level_controller (cast `/Game/Blueprints/BP_LevelController` (`GameplayStatics.GetPlayerController` 0)))
  (bind _returnvalue_2 (`Controller.K2_GetPawn` _asbp_level_controller))
  (`self.DisableInput` _returnvalue_2 null)
  ;[1 1 1] Create level start widget
  (bind _returnvalue_3 (`|CreateWidget` "/Game/Blueprints/BP_LevelWidget.BP_LevelWidget_C"))
  (`UserWidget.AddToViewport` _returnvalue_3 0)
  (`KismetSystemLibrary.Delay` 3.0)
  (bind _returnvalue_4 (`GameplayStatics.GetActorOfClass` "/Game/Blueprints/BP_PlayerCamera.BP_PlayerCamera_C"))
  ;[1 1 1] Add player camera to BaseLevel pawn
  (bind _asbp_base_level (cast `/Game/Blueprints/BP_BaseLevel` _returnvalue_2))
  (set `/Game/Blueprints/BP_BaseLevel.PlayerCamera` _returnvalue_4 _asbp_base_level)
  (`PlayerController.SetViewTargetWithBlend` _asbp_level_controller _returnvalue_4 0.0 "VTBlend_Linear" 0.0 false)
  (bind _returnvalue_5 (`GameplayStatics.GetActorOfClass` "/Game/Blueprints/BP_LevelRoot.BP_LevelRoot_C"))
  (`SceneComponent.K2_AttachToComponent` (`Actor.RootComponent` _returnvalue_5) (`Actor.RootComponent` _returnvalue_2) "None" "SnapToTarget" "SnapToTarget" "KeepRelative" false)
  (`self.EnableInput` _returnvalue_2 _asbp_level_controller)
  ;[1 1 1] Set Target Score based on number of targets in the level
  (bind _outactors (`GameplayStatics.GetAllActorsOfClass` "/Game/Blueprints/BP_Target.BP_Target_C"))
  (bind _asbp_roller_game_instance (cast `/Game/Blueprints/BP_RollerGameInstance` (`GameplayStatics.GetGameInstance`)))
  (`/Game/Blueprints/BP_RollerGameInstance.SetTargetScore` _asbp_roller_game_instance (`KismetArrayLibrary.Array_Length` _outactors)))

(event `EndGame`
  (bind _returnvalue (`|CreateWidget` "/Game/Blueprints/BP_WinWidget.BP_WinWidget_C"))
  (`UserWidget.AddToViewport` _returnvalue 0))

(fn `UserConstructionScript`)