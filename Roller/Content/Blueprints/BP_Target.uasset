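; BP_Target is a one-shot target that awards score when the player ball hits it.
; Its Hit event checks an IsActivated flag and casts the hitting actor's class to BP_PlayerBall before activating.
; Activation sets the flag, plays a sound at the target's location and swaps the TargetMesh material to SwitchableMaterial.
; It then calls IncreaseScore on BP_RollerGameInstance, which handles the score.
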(event `self.ReceiveHit`
  (params (MyComp :type "PrimitiveComponent Object Reference") (Other :type "Actor Object Reference") (OtherComp :type "PrimitiveComponent Object Reference") (bSelfMoved :type Boolean) (HitLocation :type "Vector Structure") (HitNormal :type "Vector Structure") (NormalImpulse :type "Vector Structure") (Hit :type "HitResult Structure (by ref)"))
  (if (not (`self.IsActivated`))
    (castclass `/Game/Blueprints/BP_PlayerBall` (`GameplayStatics.GetObjectClass` Other))
    (set `self.IsActivated` true)
    (`GameplayStatics.PlaySoundAtLocation` "/Engine/VREditor/Sounds/UI/Leave_Simulate.Leave_Simulate" (`self.K2_GetActorLocation`) (struct) 1.0 1.0 0.0 null null null null)
    (`PrimitiveComponent.SetMaterial` (`self.TargetMesh`) 0 (`self.SwitchableMaterial`))
    (bind _asbp_roller_game_instance (cast `/Game/Blueprints/BP_RollerGameInstance` (`GameplayStatics.GetGameInstance`)))
    (`/Game/Blueprints/BP_RollerGameInstance.IncreaseScore` _asbp_roller_game_instance)))

(fn `UserConstructionScript`)